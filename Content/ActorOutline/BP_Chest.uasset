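; BP_Chest is a chest actor that marks itself as highlighted when hovered, apparently for an outline effect.
; HoveMe and cursor-over set IsSelected, and UpdDsp switches the custom depth stencil value on the body and cover meshes.
; A short retriggerable delay then clears the highlight, so it persists only while HoveMe keeps firing.
; Cursor-end clears it immediately.
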(event Custom|HoveMe
  (Variables|Default|SetIsSelected true)
  (CallFunction|UpdDsp)
  (Utilities|FlowControl|RetriggerableDelay 0.2)
  (Variables|Default|SetIsSelected false)
  (CallFunction|UpdDsp))

(event EventBeginPlay)

(event Collision|EventActorBeginOverlap
  (params (OtherActor :type Actor%20Object%20Reference)))

(event EventTick
  (params (DeltaSeconds :type Float%20%28single-precision%29)))

(event MouseInput|EventActorBeginCursorOver
  (Variables|Default|SetIsSelected true)
  (CallFunction|UpdDsp)
  (Utilities|FlowControl|RetriggerableDelay 0.2)
  (Variables|Default|SetIsSelected false)
  (CallFunction|UpdDsp))

(event MouseInput|EventActorEndCursorOver
  (Variables|Default|SetIsSelected false)
  (CallFunction|UpdDsp)
  (Utilities|FlowControl|RetriggerableDelay 0.2)
  (Variables|Default|SetIsSelected false)
  (CallFunction|UpdDsp))

(fn ConstructionScript)

(fn UpdDsp
  (bind _chest_chest (Variables|Default|GetChest_Chest))
  (if (Variables|Default|GetIsSelected)
    (Rendering|SetCustomDepthStencilValue _chest_chest 253)
    (else
      (Rendering|SetCustomDepthStencilValue _chest_chest 0))))