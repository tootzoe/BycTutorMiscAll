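; Simple character for synced-movement play: its move input drives both itself and a linked SlaveChar, with different input scales.
; The switch-role input returns this pawn to its cached AI controller and has the player controller possess SlaveChar.
; TakeControl and RemoveControl update the label and dynamic material colour to show main or slave status.
; InitializeMe creates that material, caches the AI controller, links the partner and starts as slave.
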(event Input|EnhancedActionEvents|EnhancedInputActionIA_Move
  (params (ActionValue :type Vector%202D%20Structure) (ElapsedSeconds :type Float%20%28double-precision%29) (TriggeredSeconds :type Float%20%28double-precision%29) (InputAction :type Input%20Action%20Object%20Reference :default "/Game/SyncCharacterMovement/Input/IA_Move.IA_Move"))
  (:Triggered
    (Pawn|Input|AddMovementInput (Math|Vector|MakeVector (.y ActionValue) (.x ActionValue) 0.0) 33.0 false)
    (Pawn|Input|AddMovementInput (Variables|Default|GetSlaveChar) (Math|Vector|MakeVector (.y ActionValue) (.x ActionValue) 0.0) 3.0 false)))

(event Input|EnhancedActionEvents|EnhancedInputActionIA_SwitchRole
  (params (ActionValue :type Boolean) (ElapsedSeconds :type Float%20%28double-precision%29) (TriggeredSeconds :type Float%20%28double-precision%29) (InputAction :type Input%20Action%20Object%20Reference :default "/Game/SyncCharacterMovement/Input/IA_SwitchRole.IA_SwitchRole"))
  (CallFunction|RemoveControl)
  (CallFunction|TakeControl (Variables|Default|GetSlaveChar)))

(event EventBeginPlay)

(event Collision|EventActorBeginOverlap
  (params (OtherActor :type Actor%20Object%20Reference)))

(event EventTick
  (params (DeltaSeconds :type Float%20%28single-precision%29)))

(fn ConstructionScript)

(fn TakeControl
  (Rendering|Components|TextRender|SetText (Variables|Default|GetPawnLabel) (Utilities|Text|MakeLiteralText "Main Char"))
  (Rendering|Material|SetVectorParameterValue (Variables|Default|GetMainMaterial) "Cr" "(R=1.000000,G=0.000000,B=0.055073,A=1.000000)" :!class /Script/Engine.MaterialInstanceDynamic)
  (Pawn|Possess (Game|GetPlayerController 0) self))

(fn RemoveControl
  (Rendering|Components|TextRender|SetText (Variables|Default|GetPawnLabel) (Utilities|Text|MakeLiteralText "Slave Char"))
  (Rendering|Material|SetVectorParameterValue (Variables|Default|GetMainMaterial) "Cr" "(R=0.000000,G=0.000000,B=1.000000,A=1.000000)" :!class /Script/Engine.MaterialInstanceDynamic)
  (Pawn|Possess (Variables|Default|GetOriAIContriller) self))

(fn InitializeMe
  (params (SlaveChar :type BP%20Simple%20Character%20Object%20Reference))
  (bind _returnvalue (Rendering|Material|CreateDynamicMaterialInstance (Variables|Default|GetCube) 0 "/Game/SyncCharacterMovement/M_SimpleCharColor.M_SimpleCharColor" "None" :!class /Script/Engine.PrimitiveComponent))
  (Variables|Default|SetMainMaterial _returnvalue)
  (Variables|Default|SetOriAIContriller (AI|GetAIController self))
  (Variables|Default|SetSlaveChar SlaveChar)
  (CallFunction|RemoveControl))